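; Player pawn for an asteroid-hazard level that plays a cinematic level sequence on BeginPlay.
; Forward input moves it along the control yaw, and Rotate input turns the controller yaw.
; Overlaps on the Hit component with Asteroid-tagged actors subtract health, destroying the pawn at zero.
; A short delay debounces damage and pulses a CameraShake flag, which nothing in this graph reads.
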(event OnComponentBeginOverlap(Hit)
  (params (OverlappedComponent :type Primitive%20Component%20Object%20Reference) (OtherActor :type Actor%20Object%20Reference) (OtherComp :type Primitive%20Component%20Object%20Reference) (OtherBodyIndex :type Integer) (bFromSweep :type Boolean) (SweepResult :type Hit%20Result%20Structure%20%28by%20ref%29))
  ;[1 1 1] CameraShake
  (if (Actor|ActorHasTag OtherActor "Asteroid")
    (if (not (Variables|Default|GetHealthDecreased))
      ;[1 1 1] Health
      (Variables|Default|SetHealth (- (Variables|Default|GetHealth) 5e+01))
      (Variables|Default|SetHealthDecreased true)
      (if (<= (Variables|Default|GetHealth) 0.0)
        (Actor|DestroyActor))
      (Variables|Default|SetCameraShake true)
      (Utilities|FlowControl|Delay 0.1)
      (Variables|Default|SetCameraShake false)
      (Variables|Default|SetHealthDecreased false))))

(event EventBeginPlay
  (bind _outactor (Sequencer|Player|CreateLevelSequencePlayer "/Game/IndividualFolders/Anandaraman_Govindasami/Sequencer/Cinematics.Cinematics"))
  (Sequencer|Player|Play (Variables|/Script/LevelSequence.LevelSequenceActor|GetSequencePlayer _outactor) :!class /Script/MovieScene.MovieSceneSequencePlayer))

(event Input|AxisEvents|InputAxisForward
  (params (AxisValue :type Float%20%28single-precision%29))
  ;[1 1 1] Movement
  (Pawn|Input|AddMovementInput (Math|Vector|GetForwardVector (Math|Rotator|MakeRotator 0.0 0.0 (.yaw (Pawn|GetControlRotation :!class /Script/Engine.Pawn)))) AxisValue false))

(event Input|AxisEvents|InputAxisRotate
  (params (AxisValue :type Float%20%28single-precision%29))
  ;[1 1 1] Movement
  (Pawn|Input|AddControllerYawInput AxisValue))

(fn ConstructionScript)