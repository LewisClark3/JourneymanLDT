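; Asteroid actor, apparently a cinematics variant, that splits when an actor tagged "Projectile" overlaps its sphere.
; The overlap stores its transform, destroys the actor, then calls SpawnSmallAsteroids.
; Unless the stored scale is approximately 0.5, that function spawns two half-scale Asteroid actors at the same location, yawed to opposite sides.
; The second spawn drops the original roll and pitch.
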(event OnComponentBeginOverlap(Sphere1)
  (params (OverlappedComponent :type Primitive%20Component%20Object%20Reference) (OtherActor :type Actor%20Object%20Reference) (OtherComp :type Primitive%20Component%20Object%20Reference) (OtherBodyIndex :type Integer) (bFromSweep :type Boolean) (SweepResult :type Hit%20Result%20Structure%20%28by%20ref%29))
  (if (Actor|ActorHasTag OtherActor "Projectile")
    (Variables|Default|SetScale (Transformation|GetActorScale3D))
    (Variables|Default|SetLocation (Transformation|GetActorLocation))
    (Variables|Default|SetRotation (Transformation|GetActorRotation))
    (Actor|DestroyActor)
    (CallFunction|SpawnSmallAsteroids)))

(fn ConstructionScript)

(fn SpawnSmallAsteroids
  (bind _rotation (Variables|Default|GetRotation))
  (if (Math|Vector|NotEqual(Vector) (- (Variables|Default|GetScale) "0.500000,0.500000,0.500000") "0, 0, 0" 0.0001)
    (Game|SpawnActorfromClass "/Game/IndividualFolders/Anandaraman_Govindasami/Blueprints/Asteroid.Asteroid_C" (Math|Transform|MakeTransform (Variables|Default|GetLocation) (Math|Rotator|MakeRotator (.roll _rotation) (.pitch _rotation) (+ (.yaw _rotation) 45.0)) (/ (Variables|Default|GetScale) "2.000000,2.000000,2.000000")) "Undefined" 0 0)
    (Game|SpawnActorfromClass "/Game/IndividualFolders/Anandaraman_Govindasami/Blueprints/Asteroid.Asteroid_C" (Math|Transform|MakeTransform (Variables|Default|GetLocation) (Math|Rotator|MakeRotator 0.0 0.0 (- (.yaw _rotation) 45.0)) (/ (Variables|Default|GetScale) "2.000000,2.000000,2.000000")) "Undefined" 0 0)))